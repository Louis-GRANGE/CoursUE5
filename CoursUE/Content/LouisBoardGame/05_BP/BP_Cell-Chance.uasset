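; BP_Cell-Chance is the board game's Chance cell, a child Blueprint that fills in its on-board widget from cell data.
; Its InitWidget override calls the parent, then casts the WCCell widget to WBP_Cell-Gare, the class named for Gare cells rather than Chance.
; On a successful cast it passes the name, rectangle color and price from Data to that widget.
; The event graph and construction script add no logic.
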(fn `InitWidget`
  (bind (_data_name _data_rectanglecolor _data_description _data_price) (break `/Game/LouisBoardGame/07_Structure/S_CellData` (`self.Data`)))
  (`parent.InitWidget`)
  (bind _aswbp_cell__gare (cast `/Game/LouisBoardGame/06_Widget/WBP_Cell-Gare` (`WidgetComponent.GetUserWidgetObject` (`self.WC_Cell`))))
  (`/Game/LouisBoardGame/06_Widget/WBP_Cell-Gare.SetTitle` _aswbp_cell__gare _data_name)
  (`/Game/LouisBoardGame/06_Widget/WBP_Cell-Gare.SetColor` _aswbp_cell__gare _data_rectanglecolor)
  (`/Game/LouisBoardGame/06_Widget/WBP_Cell-Gare.SetPrice` _aswbp_cell__gare _data_price))

(fn `UserConstructionScript`
  (`parent.UserConstructionScript`))