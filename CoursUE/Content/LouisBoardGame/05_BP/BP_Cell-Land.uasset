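; BP_Cell-Land is the land cell of a board game, derived from a parent cell class that supplies its base behavior.
; It overrides InitWidget, calling the parent version and then filling the WCCell widget with title, color, description and price from its Data.
; The event graph holds only disabled default events, and the construction script just calls its parent.
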(fn `InitWidget`
  (bind _wc_cell (`self.WC_Cell`))
  (bind (_data_name _data_rectanglecolor _data_description _data_price) (break `/Game/LouisBoardGame/07_Structure/S_CellData` (`self.Data`)))
  (`parent.InitWidget`)
  (`/Game/LouisBoardGame/05_BP/WC_Cell.SetWidgetTitle` _wc_cell _data_name)
  (`/Game/LouisBoardGame/05_BP/WC_Cell.SetWidgetColor` _wc_cell _data_rectanglecolor)
  (`/Game/LouisBoardGame/05_BP/WC_Cell.SetWidgetDesc` _wc_cell _data_description)
  (`/Game/LouisBoardGame/05_BP/WC_Cell.SetWidgetPrice` _wc_cell _data_price))

(fn `UserConstructionScript`
  (`parent.UserConstructionScript`))