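; Board actor for a board game that builds the track of cells, registers itself with GM_BoardGame and handles dice throws.
; On BeginPlay it spawns one cell per DT_CellsData row, using index division and modulo to lay them out in rotated sides of ten.
; It launches all dice, sums their results and fires OnDicesCheck once all report.
; Helpers wrap movement around the loop and offset each player's position on a cell.
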(event `self.ReceiveBeginPlay`
  (bind _asgm_board_game (cast `/Game/LouisBoardGame/05_BP/GM_BoardGame` (`GameplayStatics.GetGameMode`)))
  (set `/Game/LouisBoardGame/05_BP/GM_BoardGame.BoardRef` self _asgm_board_game)
  (bind _outrownames (`DataTableFunctionLibrary.GetDataTableRowNames` "/Game/LouisBoardGame/07_Structure/DT_CellsData.DT_CellsData"))
  (for (_array_element _array_index) _outrownames
    (bind _returnvalue (`|GetDataTableRow` "/Game/LouisBoardGame/07_Structure/DT_CellsData.DT_CellsData" _array_element)
      (:`then`
        (bind _returnvalue_2 (`|SpawnActorFromClass` (`.CellType_18_C1DE3C364791BB431701F49ADDCF9CD6` (break `/Game/LouisBoardGame/07_Structure/S_CellData` _returnvalue)) (`KismetMathLibrary.MakeTransform` (0.0 0.0 0.0)) "Undefined" "OverrideRootScale" null _returnvalue null))
        (`self.K2_SetActorRotation` _returnvalue_2 (`KismetMathLibrary.MakeRotator` 0.0 0.0 (`KismetMathLibrary.Conv_IntToDouble` (* (/ _array_index 10) 90))) false)
        (bind _returnvalue_3 (`self.GetActorRightVector` _returnvalue_2))
        (`self.K2_SetActorLocation` _returnvalue_2 (+ (* (`self.GetActorForwardVector` _returnvalue_2) 2110.0) (* _returnvalue_3 (* (`KismetMathLibrary.Conv_IntToDouble` (mod _array_index 10)) 400.0)) (* _returnvalue_3 -2000.0)) false false)
        (`KismetArrayLibrary.Array_Add` (`self.Cells`) _returnvalue_2))))
  (set `self.StartCell` (`|GetArrayItem` (`self.Cells`))))

(event `LaunchDices`
  (set `self.DiceScore` 0)
  (set `self.DieCheck` 0)
  (for _array_element (`self.Dices`)
    (`/Game/LouisBoardGame/05_BP/BP_Die.LaunchDie` _array_element)))

(event `OnDieIsCheck`
  (params (Score :type Integer))
  (`/Engine/EditorBlueprintResources/StandardMacros.IncrementInt` (`self.DieCheck`)
    (:`  `
      (set `self.DiceScore` (+ Score (`self.DiceScore`)))
      (if (>= (`self.DieCheck`) (`KismetArrayLibrary.Array_Length` (`self.Dices`)))
        (`self.OnDicesCheck` (`self.DiceScore`))))))

(fn `Get Pos On Cell By Index`
  (params (IndexPlayer :type Integer) (indexCell :type Integer))
  (returns (ReturnValue :type "Vector Structure"))
  (bind _output (`|GetArrayItem` (`self.Cells`) indexCell))
  (return (+ (`self.K2_GetActorLocation` _output) (* (* IndexPlayer 60) (`self.GetActorForwardVector` _output)))))

(fn `GetPosFromCurrentPos`
  (params (Current :type Integer) (Add :type Integer))
  (returns (IndexPos :type Integer) (Ref :type "/Game/LouisBoardGame/05_BP/BP_Cell Object Reference"))
  (bind _returnvalue (mod (+ Current Add) (`KismetArrayLibrary.Array_Length` (`self.Cells`))))
  (return _returnvalue (`|GetArrayItem` (`self.Cells`) _returnvalue)))

(fn `UserConstructionScript`)