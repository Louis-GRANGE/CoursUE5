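; Board game GameMode that manages up to four player pawns and rotates turns between them.
; AddPlayer spawns a pawn on that player's spot in cell 0 through BoardRef, and RemovePlayer destroys the most recently added one.
; NextPlayerTurn wraps through the player array, making the single player controller possess the next pawn and updating its ControlledPawn reference, so all turns share one controller.
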(event `AddPlayer`
  (bind _returnvalue (`KismetArrayLibrary.Array_Length` (`self.Players`)))
  ;[0.4537 1 0] Adding Player
  (if (< _returnvalue 4)
    (bind _returnvalue_2 (`|SpawnActorFromClass` "/Game/LouisBoardGame/05_BP/Player/BP_Pawn-BoardGame.BP_Pawn-BoardGame_C" (`KismetMathLibrary.MakeTransform` (`/Game/LouisBoardGame/05_BP/BP_Board.Get Pos On Cell By Index` (`self.BoardRef`) _returnvalue 0)) "AlwaysSpawn" "OverrideRootScale" null _returnvalue null))
    (`KismetArrayLibrary.Array_Add` (`self.Players`) _returnvalue_2)))

(event `RemovePlayer`
  (bind _players (`self.Players`))
  (bind _returnvalue (`KismetArrayLibrary.Array_Length` _players))
  (bind _returnvalue_2 (- _returnvalue 1))
  ;[1 0.05156 0.04161] Remove Player
  (if (> _returnvalue 0)
    (`self.K2_DestroyActor` (`|GetArrayItem` _players _returnvalue_2))
    (`KismetArrayLibrary.Array_Remove` _players _returnvalue_2)))

(event `NextPlayerTurn`
  (bind _returnvalue (`GameplayStatics.GetPlayerController` 0))
  (bind _players (`self.Players`))
  (bind _output (`|GetArrayItem` _players (`self.IndexPlayerTurn`)))
  (bind _result (`/Engine/EditorBlueprintResources/StandardMacros.IncrementInt` (`self.IndexPlayerTurn`))
    (:`  `
      (if (not (< _result (`KismetArrayLibrary.Array_Length` _players)))
        (set `self.IndexPlayerTurn` 0))
      (`Controller.Possess` _returnvalue _output)
      (bind _asbp_player_controller__board_game (cast `/Game/LouisBoardGame/05_BP/Player/BP_PlayerController-BoardGame` _returnvalue))
      (set `/Game/LouisBoardGame/05_BP/Player/BP_PlayerController-BoardGame.ControlledPawn` _output _asbp_player_controller__board_game))))

(fn `UserConstructionScript`)