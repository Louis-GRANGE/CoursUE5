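; BP_Die is a physics-driven die for the board game that registers itself with the board shortly after BeginPlay.
; LaunchDie throws the cube with random upward and angular impulses, then a looping timer polls until it comes to rest.
; The result is read from whichever child component's forward vector points up, using its object name as the number, and is reported to the board through OnDieIsCheck.
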(event `self.ReceiveBeginPlay`
  (`KismetSystemLibrary.Delay` 0.2)
  (bind _asgm_board_game (cast `/Game/LouisBoardGame/05_BP/GM_BoardGame` (`GameplayStatics.GetGameMode`)))
  (bind _output_get (set `self.Board Ref` (`/Game/LouisBoardGame/05_BP/GM_BoardGame.BoardRef` _asgm_board_game)))
  (`KismetArrayLibrary.Array_Add` (`/Game/LouisBoardGame/05_BP/BP_Board.Dices` _output_get) self))

(event `LaunchDie`
  (bind _cube (`self.Cube`))
  (`PrimitiveComponent.AddImpulse` _cube (`KismetMathLibrary.MakeVector` 0.0 0.0 (`KismetMathLibrary.RandomFloatInRange` 600.0 1500.0)) "None" true)
  (`PrimitiveComponent.AddAngularImpulseInDegrees` _cube (* (`KismetMathLibrary.RandomUnitVector`) 750.0) "None" true)
  (bind _returnvalue (`KismetSystemLibrary.K2_SetTimerDelegate` (`|CreateDelegate` :!event `Evt_CheckIsStop`) 0.2 true))
  (set `self.CheckIsStop` _returnvalue))

(event `Evt_CheckIsStop`
  (bind _cube (`self.Cube`))
  (if (and (== (`SceneComponent.GetComponentVelocity` _cube) (0.0 0.0 0.0) :`ErrorTolerance` 1.0) (== (`PrimitiveComponent.GetPhysicsAngularVelocityInDegrees` _cube "None") (0.0 0.0 0.0) :`ErrorTolerance` 1.0))
    (`KismetSystemLibrary.K2_ClearAndInvalidateTimerHandle` (`self.CheckIsStop`))
    (bind _returnvalue (`self.GetNumber`))
    (`/Game/LouisBoardGame/05_BP/BP_Board.OnDieIsCheck` (`self.Board Ref`) _returnvalue)))

(fn `GetNumber`
  (returns (ReturnValue :type Integer))
  (for _array_element (`SceneComponent.GetChildrenComponents` (`self.Cube`) false)
    (if (== (`SceneComponent.GetForwardVector` _array_element) (`KismetMathLibrary.Vector_Up`) :`ErrorTolerance` 0.2)
      (return (`KismetStringLibrary.Conv_StringToInt` (`KismetSystemLibrary.GetObjectName` _array_element))))))

(fn `UserConstructionScript`)