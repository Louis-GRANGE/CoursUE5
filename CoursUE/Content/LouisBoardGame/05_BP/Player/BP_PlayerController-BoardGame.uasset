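; Player controller for a board game that handles joining, leaving, dice launching and pawn movement, with the mouse cursor shown.
; Join and Leave inputs add or remove players through GM_BoardGame; when the first player joins, their pawn becomes player 0's ControlledPawn.
; After a short startup delay it binds to the board's dice-check event.
; MovingByScore advances ControlledPawn by a number, placing it directly on the board-computed cell position.
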(event `self.ReceiveBeginPlay`
  (set `self.bShowMouseCursor` true)
  (`WidgetBlueprintLibrary.SetInputMode_GameAndUIEx` self null)
  (`KismetSystemLibrary.Delay` 0.2)
  (bind _asgm_board_game (cast `/Game/LouisBoardGame/05_BP/GM_BoardGame` (`GameplayStatics.GetGameMode`)))
  (bind _output_get (set `self.Board Ref` (`/Game/LouisBoardGame/05_BP/GM_BoardGame.BoardRef` _asgm_board_game)))
  (add `/Game/LouisBoardGame/05_BP/BP_Board.OnDicesCheck` _output_get (`|CreateDelegate` :!event `MovingByScore`)))

(event `InputAction|LaunchDice`
  (params (Key :type "Key Structure"))
  (:`Pressed`
    (`/Engine/EditorBlueprintResources/StandardMacros.IsValid` (`self.ControlledPawn`)
      (:`Is Valid`
        (`/Game/LouisBoardGame/05_BP/BP_Board.LaunchDices` (`self.Board Ref`))))))

(event `InputAction|Join`
  (params (Key :type "Key Structure"))
  (:`Pressed`
    (bind _asgm_board_game (cast `/Game/LouisBoardGame/05_BP/GM_BoardGame` (`GameplayStatics.GetGameMode`)))
    (`/Game/LouisBoardGame/05_BP/GM_BoardGame.AddPlayer` _asgm_board_game)
    (bind _players (`/Game/LouisBoardGame/05_BP/GM_BoardGame.Players` _asgm_board_game))
    (if (== (`KismetArrayLibrary.Array_Length` _players) 1)
      (bind _asbp_player_controller__board_game (cast `/Game/LouisBoardGame/05_BP/Player/BP_PlayerController-BoardGame` (`GameplayStatics.GetPlayerController` 0)))
      (set `/Game/LouisBoardGame/05_BP/Player/BP_PlayerController-BoardGame.ControlledPawn` (`|GetArrayItem` _players) _asbp_player_controller__board_game))))

(event `InputAction|Leave`
  (params (Key :type "Key Structure"))
  (:`Pressed`
    (bind _asgm_board_game (cast `/Game/LouisBoardGame/05_BP/GM_BoardGame` (`GameplayStatics.GetGameMode`)))
    (`/Game/LouisBoardGame/05_BP/GM_BoardGame.RemovePlayer` _asgm_board_game)))

(event `MovingByScore`
  (params (Number :type Integer))
  (bind _board_ref (`self.Board Ref`))
  (bind _controlledpawn (`self.ControlledPawn`))
  (bind _indexpos (`/Game/LouisBoardGame/05_BP/BP_Board.GetPosFromCurrentPos` _board_ref (`/Game/LouisBoardGame/05_BP/Player/BP_Pawn-BoardGame.CurrentPosOnBoard` _controlledpawn) Number))
  (set `/Game/LouisBoardGame/05_BP/Player/BP_Pawn-BoardGame.CurrentPosOnBoard` _indexpos _controlledpawn)
  (`self.K2_SetActorLocation` _controlledpawn (`/Game/LouisBoardGame/05_BP/BP_Board.Get Pos On Cell By Index` _board_ref (`/Game/LouisBoardGame/05_BP/Player/BP_Pawn-BoardGame.Index` _controlledpawn) _indexpos) false false))

(fn `UserConstructionScript`)