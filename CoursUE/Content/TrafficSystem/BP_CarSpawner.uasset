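; Traffic spawner that populates its assigned Road with a set number of cars on BeginPlay.
; Each car gets a random class and, on two-way roads, a random direction, then spawns with its road, spline distance and direction.
; GetFreePlaceInRoad picks random distances along the road spline, recursively retrying without a limit when one lands too close to an already spawned car in the same direction.
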(event `self.ReceiveBeginPlay`
  (`self.SpawnCars`))

(event `SpawnCars`
  (bind _carclasses (`self.CarClasses`))
  (for _ (range 1 (+ (`self.NbCars`) 1))
    (bind (_freeplaceonroad _invert) (`self.GetFreePlaceInRoad` (select `bool` (`/Game/TrafficSystem/BP_Road.IsTwoWay` (`self.Road`)) :`true` (`KismetMathLibrary.RandomBool`))))
    (bind _returnvalue (`|SpawnActorFromClass` (`|GetArrayItem` _carclasses (`KismetMathLibrary.RandomIntegerInRange` 0 (- (`KismetArrayLibrary.Array_Length` _carclasses) 1))) (`KismetMathLibrary.MakeTransform` (0.0 0.0 0.0)) "AlwaysSpawn" "OverrideRootScale" null (`self.Road`) _freeplaceonroad _invert null))
    (`KismetArrayLibrary.Array_Add` (`self.CarsInRoad`) _returnvalue)))

(fn `GetFreePlaceInRoad`
  (params (IsInvert :type Boolean))
  (returns (FreePlaceOnRoad :type "Float (double-precision)") (Invert :type Boolean))
  (locals (FreePlace :type "Float (double-precision)" :default 0.0))
  (bind _output_get (set `local.FreePlace` (`KismetMathLibrary.RandomFloatInRange` 0.0 (`SplineComponent.GetSplineLength` (`/Game/TrafficSystem/BP_Road.Spline` (`self.Road`))))))
  (for _array_element (`self.CarsInRoad`)
    (if (and (`KismetMathLibrary.NearlyEqual_FloatFloat` (`/Game/TrafficSystem/BP_Car.CurrentDistance` _array_element) _output_get 100.0) (== (`/Game/TrafficSystem/BP_Car.IsInvert` _array_element) IsInvert))
      (bind (_freeplaceonroad _invert) (`self.GetFreePlaceInRoad` IsInvert))
      (return _freeplaceonroad _invert)))
  (return (`local.FreePlace`) IsInvert))

(fn `UserConstructionScript`)