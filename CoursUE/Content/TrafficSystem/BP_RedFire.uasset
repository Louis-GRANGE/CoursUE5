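; Traffic light actor that cycles a cube's material color through green, orange and red phases.
; A looping timer advances the cycle, updates the state and broadcasts it through an OnChangeState dispatcher on every tick of that timer.
; The construction script snaps it onto an assigned road's spline at a set distance, optionally flipped.
; SameDirection tests whether a given direction roughly matches its arrow's forward vector.
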(event `self.ReceiveBeginPlay`
  (`KismetSystemLibrary.K2_SetTimerDelegate` (delegate `ChangeState`) 0.5 true))

(event `ChangeState`
  (bind _output_get (set `self.Timer` (+ (`self.Timer`) 0.5)))
  (if (< _output_get 5.0)
    (`MeshComponent.SetVectorParameterValueOnMaterials` (`self.Cube`) "Color" (`KismetMathLibrary.Conv_LinearColorToVector` (`self.GreenColor`)))
    (bind _output_get_2 (set `self.State` "NewEnumerator0"))
    (`self.OnChangeState` _output_get_2)
    (elif (< _output_get 7.0)
      (`MeshComponent.SetVectorParameterValueOnMaterials` (`self.Cube`) "Color" (`KismetMathLibrary.Conv_LinearColorToVector` (`self.OrangeColor`)))
      (bind _output_get_3 (set `self.State` "NewEnumerator1"))
      (`self.OnChangeState` _output_get_3)
      (elif (< _output_get 14.0)
        (`MeshComponent.SetVectorParameterValueOnMaterials` (`self.Cube`) "Color" (`KismetMathLibrary.Conv_LinearColorToVector` (`self.RedColor`)))
        (bind _output_get_4 (set `self.State` "NewEnumerator2"))
        (`self.OnChangeState` _output_get_4)
        (else
          (set `self.Timer` 0.0))))))

(fn `SameDirection`
  (params (Direction :type "Vector Structure"))
  (returns (IsSame :type Boolean))
  (return (`KismetMathLibrary.NearlyEqual_FloatFloat` (`KismetMathLibrary.Dot_VectorVector` (`SceneComponent.GetForwardVector` (`self.Arrow`)) Direction) 1.0 0.2)))

(fn `UserConstructionScript`
  (bind _attachtoroad (`self.AttachToRoad`))
  (`/Engine/EditorBlueprintResources/StandardMacros.IsValid` _attachtoroad
    (:`Is Valid`
      (`self.K2_SetActorTransform` (`KismetMathLibrary.MakeTransform` (.location (`SplineComponent.GetTransformAtDistanceAlongSpline` (`/Game/TrafficSystem/BP_Road.Spline` _attachtoroad) (`self.Distance`) "World" false)) (`KismetMathLibrary.ComposeRotators` (.rotation (`SplineComponent.GetTransformAtDistanceAlongSpline` (`/Game/TrafficSystem/BP_Road.Spline` _attachtoroad) (`self.Distance`) "World" false)) (select `bool` (`self.Invert`) :`true` (struct :`Yaw` 180.0) :!type "Rotator Structure")) (.scale (`SplineComponent.GetTransformAtDistanceAlongSpline` (`/Game/TrafficSystem/BP_Road.Spline` _attachtoroad) (`self.Distance`) "World" false)))))))