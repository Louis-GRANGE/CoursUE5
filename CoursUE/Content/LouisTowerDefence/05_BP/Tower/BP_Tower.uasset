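; Tower defence turret Blueprint that tracks BPC_AI enemies inside a radius-sized trigger and spawns bullets from its muzzle.
; Trigger overlaps maintain the target list and start or clear a looping fire-rate timer.
; Tick turns the head's yaw toward the nearest or highest-health target, and kill notifications remove targets.
; A collider supports a free-placement overlap check and switches to blocking on InitSpawn, while a range indicator scales with the radius.
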(event `self.ReceiveBeginPlay`
  (bind _radius (`self.Radius`))
  (`SphereComponent.SetSphereRadius` (`self.Trigger`) _radius true)
  (`SceneComponent.SetWorldScale3D` (`self.ShowArea`) (`KismetMathLibrary.Conv_DoubleToVector` (/ _radius 50.0))))

(event `InitSpawn`
  (`PrimitiveComponent.SetCollisionResponseToAllChannels` (`self.Collider`) "ECR_Block"))

(event `self.ReceiveTick`
  (params (DeltaSeconds :type "Float (single-precision)"))
  (if (`self.CanShoot`)
    (if (> (`KismetArrayLibrary.Array_Length` (`self.Targets`)) 0)
      (if (`self.NearTarget`)
        (bind _nearref (`self.GetNearTarget`))
        (`self.LookToTarget` (`SceneComponent.K2_GetComponentLocation` (`Actor.RootComponent` _nearref)))
        (elif (`self.MostHealth`)
          (bind _mosthealthref (`self.GetMostHeathTarget`))
          (`self.LookToTarget` (`SceneComponent.K2_GetComponentLocation` (`Actor.RootComponent` _mosthealthref))))))))

(event `self.Trigger.OnComponentBeginOverlap`
  (params (OverlappedComponent :type "PrimitiveComponent Object Reference") (OtherActor :type "Actor Object Reference") (OtherComp :type "PrimitiveComponent Object Reference") (OtherBodyIndex :type Integer) (bFromSweep :type Boolean) (SweepResult :type "HitResult Structure (by ref)"))
  (bind _asbpc_ai (cast `/Game/LouisTowerDefence/05_BP/BPC_AI` OtherActor))
  (`KismetArrayLibrary.Array_Add` (`self.Targets`) _asbpc_ai)
  (bind _returnvalue (`KismetSystemLibrary.K2_SetTimerDelegate` (`|CreateDelegate` :!event `Fire`) (`self.FireRate`) true)))

(event `self.Trigger.OnComponentEndOverlap`
  (params (OverlappedComponent :type "PrimitiveComponent Object Reference") (OtherActor :type "Actor Object Reference") (OtherComp :type "PrimitiveComponent Object Reference") (OtherBodyIndex :type Integer))
  (bind _asbpc_ai (cast `/Game/LouisTowerDefence/05_BP/BPC_AI` OtherActor))
  (`KismetArrayLibrary.Array_RemoveItem` (`self.Targets`) _asbpc_ai)
  (`KismetSystemLibrary.K2_ClearAndInvalidateTimerHandle` (stale `self.Trigger.OnComponentBeginOverlap` _returnvalue)))

(event `Fire`
  (`|SpawnActorFromClass` (`self.Bullet`) (`SceneComponent.K2_GetComponentToWorld` (`self.Muzzle`)) "Undefined" "OverrideRootScale" self (`self.Damage`) self null))

(event `HaveKillEnemy`
  (params (Ref :type "/Game/LouisTowerDefence/05_BP/BPC_AI Object Reference"))
  (`KismetArrayLibrary.Array_RemoveItem` (`self.Targets`) Ref)
  (`KismetSystemLibrary.PrintString` "Kill One" true true (struct :`R` 1.0 :`A` 1.0) 10.0))

(fn `CheckFreePlace`
  (returns (OverlappingSomethings :type Boolean))
  (bind _collider (`self.Collider`))
  (bind (_outcomponents _returnvalue) (`KismetSystemLibrary.ComponentOverlapComponents` _collider (`SceneComponent.K2_GetComponentToWorld` _collider) (`|MakeArray` "ObjectTypeQuery3" "ObjectTypeQuery2" :!type "EObjectTypeQuery Enum") null (`|MakeArray` self :!type "Actor Object Reference")))
  (return _returnvalue))

(fn `GetMostHeathTarget`
  (returns (MostHealthRef :type "/Game/LouisTowerDefence/05_BP/BPC_AI Object Reference"))
  (locals (fMostHealth :type "Float (double-precision)" :default 0.0) (MostHealthTargetRef :type "/Game/LouisTowerDefence/05_BP/BPC_AI Object Reference"))
  (for _array_element (`self.Targets`)
    (bind _health (`/Game/LouisTowerDefence/05_BP/BPC_AI.Health` _array_element))
    (if (> _health (`local.fMostHealth`))
      (set `local.fMostHealth` _health)
      (set `local.MostHealthTargetRef` _array_element)))
  (return (`local.MostHealthTargetRef`)))

(fn `GetNearTarget`
  (returns (NearRef :type "/Game/LouisTowerDefence/05_BP/BPC_AI Object Reference"))
  (locals (NearTargetRef :type "/Game/LouisTowerDefence/05_BP/BPC_AI Object Reference") (NearDistance :type "Float (double-precision)" :default 999999999999.0))
  (for _array_element (`self.Targets`)
    (bind _returnvalue (`KismetMathLibrary.Vector_Distance` (`SceneComponent.K2_GetComponentLocation` (`Actor.RootComponent` _array_element)) (`SceneComponent.K2_GetComponentLocation` (`self.DefaultSceneRoot`))))
    (if (< _returnvalue (`local.NearDistance`))
      (set `local.NearDistance` _returnvalue)
      (set `local.NearTargetRef` _array_element)))
  (return (`local.NearTargetRef`)))

(fn `LookToTarget`
  (params (Location :type "Vector Structure"))
  (bind (_returnvalue_roll _returnvalue_pitch _returnvalue_yaw) (`KismetMathLibrary.BreakRotator` (`KismetMathLibrary.FindLookAtRotation` Location (`SceneComponent.K2_GetComponentLocation` (`self.SM_Head`)))))
  (`SceneComponent.K2_SetWorldRotation` (`self.SM_Head`) (`KismetMathLibrary.MakeRotator` 0.0 0.0 (+ _returnvalue_yaw 90.0)) false false))

(fn `UserConstructionScript`
  (bind _radius (`self.Radius`))
  (`SphereComponent.SetSphereRadius` (`self.Trigger`) _radius true)
  (`SceneComponent.SetWorldScale3D` (`self.ShowArea`) (`KismetMathLibrary.Conv_DoubleToVector` (/ _radius 50.0))))