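; BP_TowerTrigger is a tower defence trigger volume that picks an AI target for a group of towers.
; When a BPC_AI overlaps the Collider it becomes the Target, and any BPC_AI leaving the volume clears it.
; Every Tick, while the Target is valid, each tower in the Towers array is told to look at the Target capsule's world location.
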(event `self.ReceiveTick`
  (params (DeltaSeconds :type "Float (single-precision)"))
  (bind _target (`self.Target`))
  (`/Engine/EditorBlueprintResources/StandardMacros.IsValid` _target
    (:`Is Valid`
      (for _array_element (`self.Towers`)
        (`/Game/LouisTowerDefence/05_BP/Tower/BP_Tower.LookToTarget` _array_element (`SceneComponent.K2_GetComponentLocation` (`Character.CapsuleComponent` _target)))))))

(event `self.Collider.OnComponentBeginOverlap`
  (params (OverlappedComponent :type "PrimitiveComponent Object Reference") (OtherActor :type "Actor Object Reference") (OtherComp :type "PrimitiveComponent Object Reference") (OtherBodyIndex :type Integer) (bFromSweep :type Boolean) (SweepResult :type "HitResult Structure (by ref)"))
  (bind _asbpc_ai (cast `/Game/LouisTowerDefence/05_BP/BPC_AI` OtherActor))
  (set `self.Target` _asbpc_ai))

(event `self.Collider.OnComponentEndOverlap`
  (params (OverlappedComponent :type "PrimitiveComponent Object Reference") (OtherActor :type "Actor Object Reference") (OtherComp :type "PrimitiveComponent Object Reference") (OtherBodyIndex :type Integer))
  (cast `/Game/LouisTowerDefence/05_BP/BPC_AI` OtherActor)
  (set `self.Target` null))

(fn `UserConstructionScript`)