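; BP_Bullet is a tower-defence projectile that damages BPC_AI enemies on trigger overlap and destroys itself after a short lifetime.
; Kills are reported back to the owning tower through TowerRef.
; On hit it either destroys itself or, without DestroyAfterHit, sticks to the enemy by attaching and disabling collision and movement.
; TakeDamage defers destruction, so the bullet destroys killed enemies last.
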(event `self.ReceiveBeginPlay`
  (`KismetSystemLibrary.Delay` 5.0)
  (`self.K2_DestroyActor`))

(event `self.Trigger.OnComponentBeginOverlap`
  (params (OverlappedComponent :type "PrimitiveComponent Object Reference") (OtherActor :type "Actor Object Reference") (OtherComp :type "PrimitiveComponent Object Reference") (OtherBodyIndex :type Integer) (bFromSweep :type Boolean) (SweepResult :type "HitResult Structure (by ref)"))
  (bind _projectilemovement (`self.ProjectileMovement`))
  (bind _asbpc_ai (cast `/Game/LouisTowerDefence/05_BP/BPC_AI` OtherActor))
  (bind _iskill (`/Game/LouisTowerDefence/05_BP/BPC_AI.TakeDamage` _asbpc_ai (`self.Damage`) false))
  (if _iskill
    (`/Game/LouisTowerDefence/05_BP/Tower/BP_Tower.HaveKillEnemy` (`self.TowerRef`) _asbpc_ai))
  (if (`self.DestroyAfterHit`)
    (`self.K2_DestroyActor`)
    (else
      (`self.K2_AttachToActor` _asbpc_ai "None" "KeepWorld" "KeepWorld" "KeepWorld")
      (`self.SetOwner` _asbpc_ai)
      (`self.SetActorEnableCollision` false)
      (`ProjectileMovementComponent.SetVelocityInLocalSpace` _projectilemovement (0.0 0.0 0.0))
      (set `ProjectileMovementComponent.bSimulationEnabled` false _projectilemovement)))
  (if _iskill
    (`self.K2_DestroyActor` _asbpc_ai)))

(fn `UserConstructionScript`)