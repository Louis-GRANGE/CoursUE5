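; BPC_AI is an AI pawn for a tower defence game that wanders the navmesh and carries health with a health bar widget.
; On BeginPlay it fills health, initialises the bar, and loops AIMoveTo toward random nearby points, pausing briefly after success or failure.
; TakeDamage broadcasts health changes and reports kills when health would drop below zero, optionally destroying the actor without updating its stored health.
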(event `self.ReceiveBeginPlay`
  (set `self.Health` (`self.MaxHealth`))
  (`|AIMoveTo` self (`NavigationSystemV1.K2_GetRandomLocationInNavigableRadius` (`NavigationSystemV1.GetNavigationSystem`) (`self.K2_GetActorLocation`) 100.0 null null) null :!label _label
    (:`then`
      (bind _aswbp_health_bar (cast `/Game/LouisTowerDefence/06_Widget/WBP_HealthBar` (`WidgetComponent.GetWidget` (`self.WBP_HealthBar`))))
      (`/Game/LouisTowerDefence/06_Widget/WBP_HealthBar.InitWidget` _aswbp_health_bar self))
    (:`OnSuccess`
      (`KismetSystemLibrary.Delay` 0.2 :!label _label_2)
      (goto _label))
    (:`OnFail`
      (goto _label_2))))

(fn `TakeDamage`
  (params (Damage :type "Float (double-precision)") (DestroyIt :type Boolean :default true))
  (returns (IsKill :type Boolean) (CurrentHealth :type "Float (double-precision)"))
  (bind _returnvalue (- (`self.Health`) Damage))
  (if (< _returnvalue 0.0)
    (`self.OnHealthChange` 0.0 (`self.MaxHealth`))
    (if DestroyIt
      (`self.K2_DestroyActor`))
    (return true _returnvalue)
    (else
      (bind _output_get (set `self.Health` _returnvalue))
      (`self.OnHealthChange` _output_get (`self.MaxHealth`))
      (return false _output_get))))

(fn `UserConstructionScript`)