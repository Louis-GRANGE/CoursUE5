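; BP_Block is a data-driven block actor for a Minecraft-style game, with its look defined by a RowName lookup in DT_Blocks.
; The construction script applies the row's mesh and material, then passes the actor's location to the material's "Location" parameter.
; BeginPlay repeats the lookup and mesh/material assignment without setting Location again.
; IsSelect toggles selection feedback through the material's "Select" scalar parameter.
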(event `self.ReceiveBeginPlay`
  (bind _staticmesh (`self.StaticMesh`))
  (bind _returnvalue (`|GetDataTableRow` "/Game/LouisMinecraft/07_Datatables/DT_Blocks.DT_Blocks" (`self.Row Name`))
    (:`then`
      (bind _output_get (set `self.Data` _returnvalue))
      (bind (_id _mesh _material) (break `/Game/LouisMinecraft/06_Structures/S_BlockData` _output_get))
      (`StaticMeshComponent.SetStaticMesh` _staticmesh _mesh)
      (`PrimitiveComponent.SetMaterial` _staticmesh 0 _material))))

(fn `IsSelect`
  (params (Select :type Boolean))
  (`MeshComponent.SetScalarParameterValueOnMaterials` (`self.StaticMesh`) "Select" (select `bool` Select :`true` 1.0 :!type "Float (single-precision)")))

(fn `UserConstructionScript`
  (bind _staticmesh (`self.StaticMesh`))
  (bind _returnvalue (`|GetDataTableRow` "/Game/LouisMinecraft/07_Datatables/DT_Blocks.DT_Blocks" (`self.Row Name`))
    (:`then`
      (bind _output_get (set `self.Data` _returnvalue))
      (bind (_id _mesh _material) (break `/Game/LouisMinecraft/06_Structures/S_BlockData` _output_get))
      (`StaticMeshComponent.SetStaticMesh` _staticmesh _mesh)
      (`PrimitiveComponent.SetMaterial` _staticmesh 0 _material)
      (`MeshComponent.SetVectorParameterValueOnMaterials` _staticmesh "Location" (`self.K2_GetActorLocation`)))))