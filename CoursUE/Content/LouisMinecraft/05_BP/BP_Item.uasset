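; BP_Item is a pickup item actor that the Minecraft-style player character collects by touching it.
; On BeginPlay it applies the mesh and material from its Data struct and sets the material's UseMovement parameter.
; When a BP_Character-MC overlaps the Trigger, it looks up Data.ID in DT_Items, passes that row's item to AddItem and destroys itself if the row is found.
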(event `self.ReceiveBeginPlay`
  (bind _staticmesh (`self.StaticMesh`))
  (bind (_id _mesh _material) (break `/Game/LouisMinecraft/07_Structures/S_BlockData` (`self.Data`)))
  (`StaticMeshComponent.SetStaticMesh` _staticmesh _mesh)
  (`PrimitiveComponent.SetMaterial` _staticmesh 0 _material)
  (`MeshComponent.SetScalarParameterValueOnMaterials` _staticmesh "UseMovement" 1.0))

(event `self.Trigger.OnComponentBeginOverlap`
  (params (OverlappedComponent :type "PrimitiveComponent Object Reference") (OtherActor :type "Actor Object Reference") (OtherComp :type "PrimitiveComponent Object Reference") (OtherBodyIndex :type Integer) (bFromSweep :type Boolean) (SweepResult :type "HitResult Structure (by ref)"))
  (bind _asbp_character__mc (cast `/Game/LouisMinecraft/05_BP/BP_Character-MC` OtherActor))
  (bind _returnvalue (`|GetDataTableRow` "/Game/LouisMinecraft/08_Datatables/DT_Items.DT_Items" (`.ID_44_CB9E4E3E422C76777E9C62BB9E737B65` (break `/Game/LouisMinecraft/07_Structures/S_BlockData` (`self.Data`))))
    (:`then`
      (`/Game/LouisMinecraft/05_BP/BP_Character-MC.AddItem` _asbp_character__mc (`.Item_8_48D90F6E40B23AED8FD722B7749FF0F6` (break `/Game/LouisMinecraft/07_Structures/S_ItemMainData` _returnvalue)))
      (`self.K2_DestroyActor`))))

(fn `UserConstructionScript`)