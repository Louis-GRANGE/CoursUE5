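; BP_Block is a Minecraft-style breakable block whose mesh, material and health come from its DT_Blocks row.
; Breaking subtracts per-tool damage, drives a material crack blend, then spawns BP_Item with the block's data and destroys itself at zero health.
; IsSelect and ResetHealth update highlight and damage material parameters, while construction passes world location to the material.
; PressDestroy and ReleaseDestroy toggle a gate whose pointed-block check leads nowhere.
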(event `self.ReceiveBeginPlay`
  (bind _staticmesh (`self.StaticMesh`))
  (bind _returnvalue (`|GetDataTableRow` "/Game/LouisMinecraft/08_Datatables/DT_Blocks.DT_Blocks" (`self.Row Name`))
    (:`then`
      (bind _output_get (set `self.Data` _returnvalue))
      (bind (_id _mesh _material _health) (break `/Game/LouisMinecraft/07_Structures/S_BlockData` _output_get))
      (`StaticMeshComponent.SetStaticMesh` _staticmesh _mesh)
      (`PrimitiveComponent.SetMaterial` _staticmesh 0 _material)
      (set `self.CurrentHealth` _health))))

(event `PressDestroy`
  (params (Player :type "/Game/LouisMinecraft/05_BP/BP_Character-MC Object Reference"))
  (`|ExecutionSequence`
    (:`then_0`
      (goto _label :!via `Open`))
    (:`then_1`
      (`/Engine/EditorBlueprintResources/StandardMacros.Gate` true :!label _label
        (:`Exit`
          (`|ExecutionSequence`
            (:`then_0`
              (if (!= (`/Game/LouisMinecraft/05_BP/BP_Character-MC.PointedBlock` Player) self)
                _))))))))

(event `ReleaseDestroy`
  (goto _label :!via `Close`))

(fn `Breaking`
  (params (PlayerTool :type "/Game/LouisMinecraft/07_Structures/E_ToolType Enum" :default "NewEnumerator0"))
  (bind ((`Health_11_FE90A10F49B1EB088197388CC4874843` _health) (`ToolDamageMadifier_19_761FCE064A9F6EB66A94D89DC84BF7B5` _tooldamagemadifier)) (break `/Game/LouisMinecraft/07_Structures/S_BlockData` (`self.Data`)))
  (bind (_value _returnvalue) (`BlueprintMapLibrary.Map_Find` _tooldamagemadifier PlayerTool))
  (bind _output_get (set `self.CurrentHealth` (- (`self.CurrentHealth`) (select `bool` _returnvalue :`false` 1.0 :`true` _value))))
  (`MeshComponent.SetScalarParameterValueOnMaterials` (`self.StaticMesh`) "BreakingLerp" (`KismetMathLibrary.MapRangeClamped` _output_get 0.0 _health 1.0 0.0))
  (if (<= _output_get 0.0)
    (`/Engine/EditorBlueprintResources/StandardMacros.DoOnce` false
      (:`Completed`
        (`|SpawnActorFromClass` "/Game/LouisMinecraft/05_BP/BP_Item.BP_Item_C" (`KismetMathLibrary.MakeTransform` (`SceneComponent.K2_GetComponentLocation` (`self.DefaultSceneRoot`))) "Undefined" "OverrideRootScale" null (`self.Data`) null)
        (`self.K2_DestroyActor`)))))

(fn `IsSelect`
  (params (Select :type Boolean))
  (`MeshComponent.SetScalarParameterValueOnMaterials` (`self.StaticMesh`) "Select" (select `bool` Select :`true` 1.0 :!type "Float (single-precision)")))

(fn `ResetHealth`
  (set `self.CurrentHealth` (`.Health_11_FE90A10F49B1EB088197388CC4874843` (break `/Game/LouisMinecraft/07_Structures/S_BlockData` (`self.Data`))))
  (`MeshComponent.SetScalarParameterValueOnMaterials` (`self.StaticMesh`) "BreakingLerp" 0.0))

(fn `UserConstructionScript`
  (bind _staticmesh (`self.StaticMesh`))
  (bind _returnvalue (`|GetDataTableRow` "/Game/LouisMinecraft/08_Datatables/DT_Blocks.DT_Blocks" (`self.Row Name`))
    (:`then`
      (bind _output_get (set `self.Data` _returnvalue))
      (bind (_id _mesh _material) (break `/Game/LouisMinecraft/07_Structures/S_BlockData` _output_get))
      (`StaticMeshComponent.SetStaticMesh` _staticmesh _mesh)
      (`PrimitiveComponent.SetMaterial` _staticmesh 0 _material)
      (`MeshComponent.SetVectorParameterValueOnMaterials` _staticmesh "Location" (`self.K2_GetActorLocation`)))))