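; BP_TriggerButton is a trigger volume that sends linked elevators up or down when the player character steps into it.
; When a BP_Character overlaps the Box, it calls MoveTo on every entry in the Elevator array, passing its MoveUp flag.
; A TextRender labels the button "Up" or "Down" from that flag, set in both the construction script and BeginPlay.
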(event `self.ReceiveBeginPlay`
  (`TextRenderComponent.K2_SetText` (`self.TextRender`) (`|FormatText` (select `bool` (`self.MoveUp`) :`false` "Down" :`true` "Up" :!type "Text"))))

(event `self.Box.OnComponentBeginOverlap`
  (params (OverlappedComponent :type "PrimitiveComponent Object Reference") (OtherActor :type "Actor Object Reference") (OtherComp :type "PrimitiveComponent Object Reference") (OtherBodyIndex :type Integer) (bFromSweep :type Boolean) (SweepResult :type "HitResult Structure (by ref)"))
  (cast `/Game/Louis/BP_Character` OtherActor)
  (for _array_element (`self.Elevator`)
    (`/Game/Louis/BP_Elevator.MoveTo` _array_element (`self.MoveUp`))))

(fn `UserConstructionScript`
  (`TextRenderComponent.K2_SetText` (`self.TextRender`) (`|FormatText` (select `bool` (`self.MoveUp`) :`false` "Down" :`true` "Up" :!type "Text"))))