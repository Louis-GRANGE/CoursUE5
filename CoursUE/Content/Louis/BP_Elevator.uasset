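; Elevator actor that moves its FloorScene platform one floor up or down between evenly spaced stops built on BeginPlay.
; MoveTo applies the Inverted flag, checks floor bounds, then starts a looping timer that runs MoveToPoint to lerp the transform and drive Cube's emissive colour by direction.
; The construction script labels it Normal or Invert.
; Separate GoUp/GoDown functions instantly step the whole actor, uncalled in this graph.
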(event `self.ReceiveBeginPlay`
  (`KismetArrayLibrary.Array_Clear` (`self.Floors`))
  (for _index (range (`self.NbFloor`))
    (`KismetArrayLibrary.Array_Add` (`self.Floors`) (`KismetMathLibrary.MakeTransform` (+ (`self.K2_GetActorLocation`) (`KismetMathLibrary.MakeVector` 0.0 0.0 (* _index (`self.Step/Amount`))))))))

(event `MoveTo`
  (params (DirectionUP :type Boolean))
  (bind _returnvalue (select `bool` (`self.Inverted`) :`false` DirectionUP :`true` (not DirectionUP)))
  (bind _returnvalue_2 (+ (`self.CurrentFloor`) (select `bool` _returnvalue :`false` -1 :`true` 1)))
  (set `self.bGoUp` _returnvalue)
  (if (and (< _returnvalue_2 (`KismetArrayLibrary.Array_Length` (`self.Floors`))) (>= _returnvalue_2 0))
    (bind _output_get (set `self.CurrentFloor` _returnvalue_2))
    (set `self.PointToGo` (`|GetArrayItem` (`self.Floors`) _output_get))
    (set `self.CurrentLocation` (`SceneComponent.K2_GetComponentToWorld` (`self.FloorScene`)))
    (set `self.TimeLerp` 0.0)
    (bind _returnvalue_3 (`KismetSystemLibrary.K2_SetTimer` null "MoveToPoint" 0.01 true))
    (set `self.Moving` _returnvalue_3)))

(fn `GoDown`
  (`self.MoveToDirection` (* (`self.GetActorUpVector`) -1.0))
  (set `self.bGoUp` false))

(fn `GoUp`
  (`self.MoveToDirection` (`self.GetActorUpVector`))
  (set `self.bGoUp` true))

(fn `MoveToDirection`
  (params (Direction :type "Vector Structure"))
  (`self.K2_SetActorLocation` (+ (* (`KismetMathLibrary.Normal` Direction) (`self.Step/Amount`)) (`self.K2_GetActorLocation`))))

(fn `MoveToPoint`
  (bind _cube (`self.Cube`))
  (bind _cube_2 (`self.Cube`))
  (bind _timelerp (`self.TimeLerp`))
  (`MeshComponent.SetScalarParameterValueOnMaterials` _cube "Lerp" _timelerp)
  (`MeshComponent.SetVectorParameterValueOnMaterials` _cube "EmissiveB" (`KismetMathLibrary.Conv_LinearColorToVector` (select `bool` (`self.bGoUp`) :`false` (`self.ColorDown`) :`true` (`self.ColorUp`))))
  (`SceneComponent.K2_SetWorldTransform` (`self.FloorScene`) (`KismetMathLibrary.TLerp` (`self.CurrentLocation`) (`self.PointToGo`) _timelerp) false false)
  (bind _output_get (set `self.TimeLerp` (+ (/ 0.01 (`self.TimeToGo`)) (`self.TimeLerp`))))
  (if (>= _output_get 1.0)
    (`MeshComponent.SetVectorParameterValueOnMaterials` _cube_2 "EmissiveA" (`KismetMathLibrary.Conv_LinearColorToVector` (`self.ColorNoMove`)))
    (`MeshComponent.SetScalarParameterValueOnMaterials` _cube_2 "Lerp" 0.0)
    (`KismetSystemLibrary.K2_ClearAndInvalidateTimerHandle` (`self.Moving`))))

(fn `UserConstructionScript`
  (`TextRenderComponent.K2_SetText` (`self.TextRender`) (`|FormatText` (select `bool` (`self.Inverted`) :`false` "Normal" :`true` "Invert" :!type "Text"))))